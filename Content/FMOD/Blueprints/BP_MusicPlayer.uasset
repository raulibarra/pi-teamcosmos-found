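; Music player Blueprint that starts and steers the game's FMOD music through global parameters.
; Initialize runs once, loading the Master bank, playing the MusicPlayer event in 2D, storing its instance and setting a starting game state.
; SetGameState converts main and sub state enums to floats for the MusicState and WinState parameters.
; SetAttention passes a percentage to the Attention parameter.
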(fn Initialize
  (if (not (Variables|Default|GetIsInitialized))
    (Class|FMODBlueprintStatics|LoadBank "/Game/FMOD/Banks/Master.Master" true false)
    (bind _returnvalue (Class|FMODBlueprintStatics|PlayEvent2D "/Game/FMOD/Events/MusicPlayer.MusicPlayer"))
    (Variables|Default|SetAudioInstance _returnvalue)
    (Variables|Default|SetIsInitialized true)
    (CallFunction|SetGameState "NewEnumerator1" "NewEnumerator0")))

(fn SetGameState
  (params (MainState :type EMusicState%20Enum :default "NewEnumerator1") (SubState :type EWinState%20Enum :default "NewEnumerator0"))
  (Class|FMODBlueprintStatics|SetGlobalParameterbyName "MusicState" (Math|Conversions|ToFloat(Byte) MainState))
  (Class|FMODBlueprintStatics|SetGlobalParameterbyName "WinState" (Math|Conversions|ToFloat(Byte) SubState)))

(fn SetAttention
  (params (AttentionPercent :type Float%20%28single-precision%29))
  (Class|FMODBlueprintStatics|SetGlobalParameterbyName "Attention" AttentionPercent))